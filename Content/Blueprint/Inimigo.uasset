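; Inimigo is an enemy actor that damages the player on contact and is destroyed when it dies.
; On BeginPlay it moves the AreaDano volume to the mesh socket of the same name, scales it down and attaches it there.
; Overlaps send a fixed AlterarVida message to player-tagged actors implementing ISofrerDano.
; Its own AlterarVida event runs CalcularVida and destroys the actor if IsDead is set.
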(event `/Game/Blueprint/iSofrerDano.AlterarVida`
  (params (delta :type "Float (single-precision)"))
  (`self.CalcularVida` delta)
  (if (`self.isDead`)
    (`self.K2_DestroyActor`)))

(event `self.ReceiveBeginPlay`
  (`SceneComponent.K2_SetWorldTransform` (`self.AreaDano`) (`SceneComponent.GetSocketTransform` (`self.Mesh`) "AreaDano" "RTS_World") false false)
  (`SceneComponent.SetWorldScale3D` (`self.AreaDano`) (0.4 0.4 0.4))
  (`SceneComponent.K2_AttachToComponent` (`self.AreaDano`) (`self.Mesh`) "AreaDano" "KeepWorld" "KeepWorld" "KeepWorld" true))

(event `self.AreaDano.OnComponentBeginOverlap`
  (params (OverlappedComponent :type "PrimitiveComponent Object Reference") (OtherActor :type "Actor Object Reference") (OtherComp :type "PrimitiveComponent Object Reference") (OtherBodyIndex :type Integer) (bFromSweep :type Boolean) (SweepResult :type "HitResult Structure (by ref)"))
  (if (`KismetSystemLibrary.DoesImplementInterface` OtherActor "/Game/Blueprint/iSofrerDano.iSofrerDano_C")
    (if (`self.ActorHasTag` OtherActor "player")
      (message `/Game/Blueprint/iSofrerDano.AlterarVida` OtherActor 1.0))))

(fn `UserConstructionScript`)
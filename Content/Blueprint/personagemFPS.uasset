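; First-person shooter player character (personagemFPS) that moves, turns, jumps, fires a weapon and can die.
; Movement axes follow control rotation and horizontal look adds yaw, while the LookUp axis is left unconnected.
; BeginPlay sets maximum life and spawns an ArmaPersonagem weapon on the mesh's ArmaSocket, which left click fires through Atirar.
; AlterarVida passes health changes to CalcularVida and destroys the actor when IsDead is set.
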(event `InputAxis|MoveForward`
  (params (AxisValue :type "Float (single-precision)"))
  ;[1 1 1] Movimentação do Jogador
  (`self.AddMovementInput` (`KismetMathLibrary.GetForwardVector` (`self.GetControlRotation`)) AxisValue))

(event `InputAxis|LookUp`
  (params (AxisValue :type "Float (single-precision)"))
  ;[1 1 1] Rotação Jogador
)

(event `InputAxis|MoveRight`
  (params (AxisValue :type "Float (single-precision)"))
  ;[1 1 1] Movimentação do Jogador
  (`self.AddMovementInput` (`KismetMathLibrary.GetRightVector` (`self.GetControlRotation`)) AxisValue))

(event `InputAxis|LookRight`
  (params (AxisValue :type "Float (single-precision)"))
  ;[1 1 1] Rotação Jogador
  (`self.AddControllerYawInput` AxisValue))

(event `Key|SpaceBar`
  (params (Key :type "Key Structure"))
  ;[1 1 1] Pulo
  (:`Pressed`
    (`self.Jump`)))

(event `self.ReceiveBeginPlay`
  (bind _mesh (`self.Mesh`))
  ;[1 1 1] Comment
  (`|ExecutionSequence`
    (:`then_0`
      (set `self.lifeMax` 100.0))
    (:`then_1`
      (bind _returnvalue (`|SpawnActorFromClass` "/Game/Blueprint/ArmaPersonagem.ArmaPersonagem_C" (`SceneComponent.GetSocketTransform` _mesh "ArmaSocket" "RTS_World") "Undefined" "OverrideRootScale" null null))
      (bind _output_get (set `self.Arma` _returnvalue))
      (`self.K2_AttachToComponent` _output_get _mesh "ArmaSocket" "KeepWorld" "KeepWorld" "KeepWorld" true))))

(event `Key|LeftMouseButton`
  (params (Key :type "Key Structure"))
  ;[1 1 1] usar Arma
  (:`Pressed`
    (bind _asarma_personagem (cast `/Game/Blueprint/ArmaPersonagem` (`self.Arma`)))
    (`/Game/Blueprint/ArmaPersonagem.Atirar` _asarma_personagem)))

(event `/Game/Blueprint/iSofrerDano.AlterarVida`
  (params (delta :type "Float (single-precision)"))
  ;[1 1 1] Verificar vida
  (`self.CalcularVida` delta)
  (if (`self.isDead`)
    (`self.K2_DestroyActor`)))

(fn `UserConstructionScript`)